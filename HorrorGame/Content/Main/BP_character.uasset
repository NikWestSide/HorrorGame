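; BP_character is a player character Blueprint with axis-driven movement, look controls and a switch between first- and third-person views.
; Movement input follows the capsule's forward and right vectors, while look input feeds controller pitch and yaw.
; ChangeCamera uses a FlipFlop to swap MaimCamera and ExtraCamera, enabling controller-yaw body rotation only while ExtraCamera is active.
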(event Input|ActionEvents|InputActionChangeCamera
  (params (Key :type Key%20Structure :default "None"))
  ;[1 1 1] Вид камеры от 1 лица и 3 лица
  (:Pressed
    (Utilities|FlowControl|FlipFlop
      (:A
        (Components|Activation|Deactivate (Variables|Default|GetMaimCamera))
        (Components|Activation|Activate (Variables|Default|GetExtraCamera) false)
        (Variables|Default|SetbUseControllerRotationYaw true))
      (:B
        (Components|Activation|Deactivate (Variables|Default|GetExtraCamera))
        (Components|Activation|Activate (Variables|Default|GetMaimCamera) false)
        (Variables|Default|SetbUseControllerRotationYaw false)))))

(event Input|AxisEvents|InputAxisMoveForwardBack
  (params (AxisValue :type Float%20%28single-precision%29))
  ;[1 1 1] Передвежение
  (Pawn|Input|AddMovementInput (Math|Vector|GetForwardVector (Variables|Collision|GetCapsuleComponent)) AxisValue false))

(event Input|AxisEvents|InputAxisMoveRightLeft
  (params (AxisValue :type Float%20%28single-precision%29))
  ;[1 1 1] Передвежение
  (Pawn|Input|AddMovementInput (Math|Vector|GetRightVector (Variables|Collision|GetCapsuleComponent)) AxisValue false))

(event Input|AxisEvents|InputAxisLookUpDown
  (params (AxisValue :type Float%20%28single-precision%29))
  ;[1 1 1] Вращение камеры
  (Pawn|Input|AddControllerPitchInput AxisValue))

(event Input|AxisEvents|InputAxisLookLeftRight
  (params (AxisValue :type Float%20%28single-precision%29))
  ;[1 1 1] Вращение камеры
  (Pawn|Input|AddControllerYawInput AxisValue))

(fn ConstructionScript)