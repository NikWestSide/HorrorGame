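; Player character Blueprint handling walking, strafing, sprinting, mouse-look style camera rotation and a first/third-person view toggle.
; Axis events move along the capsule's vectors; the forward axis also resets walk speed through an ordered Sequence where backpedal overrides strafe, which overrides sprint.
; Sprint engages only if forward input is full when pressed.
; A FlipFlop swaps the two cameras and toggles controller-yaw rotation.
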(event Input|ActionEvents|InputActionChangeCamera
  (params (Key :type Key%20Structure :default "None"))
  ;[1 1 1] Вид камеры от 1 лица и 3 лица
  (:Pressed
    (Utilities|FlowControl|FlipFlop
      (:A
        (Components|Activation|Deactivate (Variables|Default|GetMaimCamera))
        (Components|Activation|Activate (Variables|Default|GetExtraCamera) false)
        (Variables|Default|SetbUseControllerRotationYaw true))
      (:B
        (Components|Activation|Deactivate (Variables|Default|GetExtraCamera))
        (Components|Activation|Activate (Variables|Default|GetMaimCamera) false)
        (Variables|Default|SetbUseControllerRotationYaw false)))))

(event Input|ActionEvents|InputActionSprint
  (params (Key :type Key%20Structure :default "None"))
  ;[1 1 1] Кнопка Бега
  (:Pressed
    (if (== (stale Input|AxisEvents|InputAxisMoveForwardBack AxisValue) 1.0)
      (Variables|Default|SetIsSprinting? true)
      (else
        (Variables|Default|SetIsSprinting? false))))
  (:Released
    (Variables|Default|SetIsSprinting? false)))

(event Input|AxisEvents|InputAxisMoveForwardBack
  (params (AxisValue :type Float%20%28single-precision%29))
  (bind _charactermovement (Variables|Character|GetCharacterMovement))
  ;[1 1 1] Передвежение
  (Pawn|Input|AddMovementInput (Math|Vector|GetForwardVector (Variables|Collision|GetCapsuleComponent)) AxisValue false)
  (Utilities|FlowControl|Sequence
    (:then_0
      (Variables|/Script/Engine.CharacterMovementComponent|SetMaxWalkSpeed _charactermovement 3e+02))
    (:then_1
      (if (== AxisValue -1.0)
        (Variables|/Script/Engine.CharacterMovementComponent|SetMaxWalkSpeed _charactermovement 1.5e+02)))
    (:then_2
      (if (Variables|Default|GetIsSprinting?)
        (Variables|/Script/Engine.CharacterMovementComponent|SetMaxWalkSpeed _charactermovement 6e+02)))
    (:then_3
      ;;[1 1 1] Скорость стрейфа
      (if (Variables|Default|GetIsWalkRightLeft)
        (Variables|/Script/Engine.CharacterMovementComponent|SetMaxWalkSpeed (Variables|Character|GetCharacterMovement) 3e+02)))
    (:then_4
      ;;[1 1 1] скорость ходьбы назад
      (if (== AxisValue -1.0)
        (Variables|/Script/Engine.CharacterMovementComponent|SetMaxWalkSpeed (Variables|Character|GetCharacterMovement) 1.5e+02)))))

(event Input|AxisEvents|InputAxisMoveRightLeft
  (params (AxisValue :type Float%20%28single-precision%29))
  ;[1 1 1] Передвежение
  (Pawn|Input|AddMovementInput (Math|Vector|GetRightVector (Variables|Collision|GetCapsuleComponent)) AxisValue false)
  (Variables|Default|SetIsWalkRightLeft (or (== AxisValue -1.0) (== AxisValue 1.0))))

(event Input|AxisEvents|InputAxisLookUpDown
  (params (AxisValue :type Float%20%28single-precision%29))
  ;[1 1 1] Вращение камеры
  (Pawn|Input|AddControllerPitchInput AxisValue))

(event Input|AxisEvents|InputAxisLookLeftRight
  (params (AxisValue :type Float%20%28single-precision%29))
  ;[1 1 1] Вращение камеры
  (Pawn|Input|AddControllerYawInput AxisValue))

(fn ConstructionScript)